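; Base character Blueprint that shows a 2D sprite with switchable expressions for Neutral, Fever and Miss states.
; The construction script starts CharSprite on the neutral sprite.
; SetEmotion switches on the given emotion and swaps CharSprite to the matching sprite variable.
; The event graph holds no logic, so emotion changes depend on calls to SetEmotion.
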(event EventBeginPlay)

(event Collision|EventActorBeginOverlap
  (params (OtherActor :type Actor%20Object%20Reference)))

(event EventTick
  (params (DeltaSeconds :type Float%20%28single-precision%29)))

(fn ConstructionScript
  (Rendering|Components|Sprite|SetSprite (Variables|Default|GetCharSprite) (Variables|Default|GetSprite_Neutral)))

(fn SetEmotion
  (params (Emotion :type E_DanceState%20Enum :default "NewEnumerator0"))
  (bind _charsprite (Variables|Default|GetCharSprite))
  (switch Utilities|FlowControl|Switch|SwitchonE_DanceState Emotion
    (:NewEnumerator0
      (Rendering|Components|Sprite|SetSprite _charsprite (Variables|Default|GetSprite_Neutral)))
    (:NewEnumerator1
      (Rendering|Components|Sprite|SetSprite _charsprite (Variables|Default|GetSprite_Fever)))
    (:NewEnumerator2
      (Rendering|Components|Sprite|SetSprite _charsprite (Variables|Default|GetSprite_Miss)))))